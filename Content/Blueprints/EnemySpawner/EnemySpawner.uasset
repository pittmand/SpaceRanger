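; Enemy spawner that populates a volume with AI-controlled enemy ships up to a MaxEnemy cap.
; Tick runs through a spawn-rate Delay into SpawnEnemy; a trailing EnemyIncreaseRate Delay leads to nothing.
; SpawnEnemy counts EnemyShip actors and, below the cap, spawns at a random point in SpawnVolume.
; A random roll up to MaxEnemy picks EnemyShip below 20, otherwise EnemyChild_Aggressive.
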(event `self.ReceiveTick`
  (params (DeltaSeconds :type "Float (single-precision)"))
  (`KismetSystemLibrary.Delay` (`self.EnemySpawnRate`))
  (`self.SpawnEnemy`)
  (`KismetSystemLibrary.Delay` (`self.EnemyIncreaseRate`)))

(event `SpawnEnemy`
  (bind _spawnvolume (`self.SpawnVolume`))
  (bind _returnvalue (`KismetMathLibrary.RandomPointInBoundingBox` (`SceneComponent.K2_GetComponentLocation` _spawnvolume) (`BoxComponent.GetScaledBoxExtent` _spawnvolume)))
  (bind _outactors (`GameplayStatics.GetAllActorsOfClass` "/Game/FlyingBP/Blueprints/EnemyShip.EnemyShip_C"))
  (if (< (`KismetArrayLibrary.Array_Length` _outactors) (`self.MaxEnemy`))
    (if (< (`KismetMathLibrary.RandomIntegerInRange` 0 (`self.MaxEnemy`)) 20)
      (`AIBlueprintHelperLibrary.SpawnAIFromClass` "/Game/FlyingBP/Blueprints/EnemyShip.EnemyShip_C" null _returnvalue)
      (else
        (`AIBlueprintHelperLibrary.SpawnAIFromClass` "/Game/FlyingBP/Blueprints/EnemyChild_Aggressive.EnemyChild_Aggressive_C" null _returnvalue)))))

(fn `UserConstructionScript`)