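; BP_Guns is a gun that fires BP_BarrierBullet projectiles at the player's FlyingPawn.
; BarrierFire waits briefly, then spawns an enlarged, limited-lifespan bullet at GunLocation.
; It leads the target by rotating the pawn's forward speed along its Weapon rotation and scaling by estimated travel time, derived from distance over a fixed divisor.
; The event's Player input is unused, as the target is always player pawn 0.
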(event `BarrierFire`
  (params (Player :type "Pawn Object Reference"))
  (bind _returnvalue (`SceneComponent.K2_GetComponentLocation` (`self.GunLocation`)))
  (`KismetSystemLibrary.Delay` 0.1)
  (bind _asflying_pawn (cast `/Game/FlyingBP/Blueprints/Player/FlyingPawn` (`GameplayStatics.GetPlayerPawn` 0)))
  (bind _returnvalue_2 (`self.K2_GetActorLocation` _asflying_pawn))
  (bind _returnvalue_3 (`|SpawnActorFromClass` "/Game/Blueprints/BP_BarrierBullet.BP_BarrierBullet_C" (`KismetMathLibrary.MakeTransform` _returnvalue (`KismetMathLibrary.FindLookAtRotation` _returnvalue (+ (* (`KismetMathLibrary.GreaterGreater_VectorRotator` (`KismetMathLibrary.MakeVector` (`/Game/FlyingBP/Blueprints/Player/FlyingPawn.Current forward speed` _asflying_pawn)) (`SceneComponent.K2_GetComponentRotation` (`/Game/FlyingBP/Blueprints/Player/FlyingPawn.weapon` _asflying_pawn))) (/ (`KismetMathLibrary.VSize` (- _returnvalue_2 (`SceneComponent.K2_GetComponentLocation` (`self.GunLocation`)))) 100000.0)) _returnvalue_2)) (5.0 5.0 5.0)) "AdjustIfPossibleButAlwaysSpawn" "OverrideRootScale" null null))
  (`self.SetLifeSpan` _returnvalue_3 15.0))

(fn `UserConstructionScript`)