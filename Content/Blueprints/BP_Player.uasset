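; BP_Player is the player actor, with a spawn animation and axis-driven horizontal and vertical movement.
; On BeginPlay it caches BP_GameMode, then a timeline lifts and spins it before setting MoveEnabled, which these graphs never read.
; MoveUp and MoveRight inputs set Z and X speeds.
; Tick does a swept move to the current location multiplied by that speed vector, rather than offset by it, and without delta-time scaling.
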(event `self.ReceiveBeginPlay`
  (bind _spawnlocation (`self.SpawnLocation`))
  (bind _asbp_game_mode (cast `/Game/Blueprints/BP_GameMode` (`GameplayStatics.GetGameMode`)))
  (set `self.BP_GameMode` _asbp_game_mode)
  (set `self.Yaw` (.yaw (`self.K2_GetActorRotation`)))
  (set `self.SpawnLocation` (`self.K2_GetActorLocation`))
  (bind (_direction _speed) (`Timeline|SpawnAnimation`)
    (:`Update`
      (`self.K2_SetActorLocation` (`KismetMathLibrary.VLerp` _spawnlocation (+ _spawnlocation (0.0 0.0 60.0)) _speed))
      (`self.K2_SetActorRotation` (`KismetMathLibrary.RLerp` (struct) (`KismetMathLibrary.MakeRotator` 0.0 0.0 (+ (`self.Yaw`) 1440.0)) _speed)))
    (:`Finished`
      (set `self.MoveEnabled` true))))

(event `self.ReceiveTick`
  (params (DeltaSeconds :type "Float (single-precision)"))
  (set `self.ElapsedTime` DeltaSeconds)
  (`self.K2_SetActorLocation` (* (`self.K2_GetActorLocation`) (`KismetMathLibrary.MakeVector` (`self.HorizontalSpeed`) 0.0 (`self.VeriticalSpeed`))) true))

(event `InputAxis|MoveUp`
  (params (AxisValue :type "Float (single-precision)"))
  (set `self.VeriticalSpeed` (* (`self.MovementSpeed`) AxisValue)))

(event `InputAxis|MoveRight`
  (params (AxisValue :type "Float (single-precision)"))
  (set `self.HorizontalSpeed` (* (`self.MovementSpeed`) AxisValue)))

(fn `UserConstructionScript`)