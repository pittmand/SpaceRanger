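; BP_SafeZone marks the area the player must stay in, punishing those who leave with gun fire.
; It polls every Tick whether the player pawn overlaps it, clearing the Return widget and AsteroidAlarm while inside.
; Leaving after being safe shows the warning, sounds the alarm and starts a countdown Delay.
; If the player is still outside afterwards, every BP_Guns actor calls BarrierFire on them each Tick until they return.
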(event `self.ReceiveTick`
  (params (DeltaSeconds :type "Float (single-precision)"))
  (bind _returnvalue (`GameplayStatics.GetPlayerPawn` 0))
  (bind _returnvalue_2 (`self.IsOverlappingActor` _returnvalue self))
  ;[1 1 1] Check For Player
  (if (`KismetSystemLibrary.IsValid` _returnvalue)
    (if _returnvalue_2
      (set `self.WasSafe` true :!label _label)
      (bind _foundwidgets (`WidgetBlueprintLibrary.GetAllWidgetsOfClass` "/Game/Blueprints/Return.Return_C"))
      (bind _output (`|GetArrayItem` _foundwidgets))
      (if (`KismetSystemLibrary.IsValid` _output)
        (`Widget.RemoveFromParent` _output))
      (`ActorComponent.Deactivate` (`self.AsteroidAlarm`))
      (elif (`self.WasSafe`)
        (bind _foundwidgets_2 (`WidgetBlueprintLibrary.GetAllWidgetsOfClass` "/Game/Blueprints/Return.Return_C"))
        (if (== (`KismetArrayLibrary.Array_Length` _foundwidgets_2) 0)
          (bind _returnvalue_3 (`|CreateWidget` "/Game/Blueprints/Return.Return_C"))
          (`UserWidget.AddToViewport` _returnvalue_3 0)
          (`ActorComponent.Activate` (`self.AsteroidAlarm`) false)
          (`KismetSystemLibrary.Delay` (`self.Countdown`))
          (if _returnvalue_2
            (goto _label)
            (else
              (set `self.WasSafe` false)
              (bind _outactors (`GameplayStatics.GetAllActorsOfClass` "/Game/Blueprints/BP_Guns.BP_Guns_C" :!label _label_2))
              (for _array_element _outactors
                (`/Game/Blueprints/BP_Guns.BarrierFire` _array_element (`GameplayStatics.GetPlayerPawn` 0))))))
        (else
          (goto _label_2))))))

(fn `UserConstructionScript`)